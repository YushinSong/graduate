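; BP_Hihgb is an alcohol Blueprint, apparently for a highball, with three progress bar components.
; Its Construction Script creates a dynamic material instance on each bar from that bar's own highball material and caches it in a variable.
; Nothing in this file drives those materials: the event graph holds only disabled default events, and the parent Construction Script call never runs.
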(event EventBeginPlay
  (|CallParentFunction) ; 지금 이 노드는 비활성 상태입니다. \n핀을 끌어서 다른 노드를 연결하면 활성화됩니다.
)

(event Collision|EventActorBeginOverlap
  (params (OtherActor :type Actor%20Object%20Reference))
  (|CallParentFunction OtherActor) ; 지금 이 노드는 비활성 상태입니다. \n핀을 끌어서 다른 노드를 연결하면 활성화됩니다.
)

(event EventTick
  (params (DeltaSeconds :type Float%20%28single-precision%29))
  (|CallParentFunction DeltaSeconds) ; 지금 이 노드는 비활성 상태입니다. \n핀을 끌어서 다른 노드를 연결하면 활성화됩니다.
)

(fn ConstructionScript
  (bind _returnvalue (Rendering|Material|CreateDynamicMaterialInstance (Variables|Default|GetProgressBar) 0 "/Game/Interface/MI_HighballPBar1.MI_HighballPBar1" :!class /Script/Engine.PrimitiveComponent))
  (Variables|Default|SetProgressMI1 _returnvalue)
  (bind _returnvalue_2 (Rendering|Material|CreateDynamicMaterialInstance (Variables|Default|GetProgressBar2) 0 "/Game/Interface/MI_HighballPBar2.MI_HighballPBar2" :!class /Script/Engine.PrimitiveComponent))
  (Variables|Default|SetProgressMI2 _returnvalue_2)
  (bind _returnvalue_3 (Rendering|Material|CreateDynamicMaterialInstance (Variables|Default|GetProgressBar3) 0 "/Game/Interface/MI_HighballPBar3.MI_HighballPBar3" :!class /Script/Engine.PrimitiveComponent))
  (Variables|Default|SetProgressMI3 _returnvalue_3))