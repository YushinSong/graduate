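; Old Fashioned drink actor that shows up to three poured ingredients as colored, labeled fill levels.
; While IsClicked, Tick raises the bar for the current DrinkNum and every later one through dynamic material instances, colored from DrinksColorMap by DrinkName.
; Each ingredient's percentage is its bar minus the previous one, shown on a text label that rises with the fill.
; CheckPercent flags a total above 99, which stops label updates and clears IsClicked.
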(event Custom|Check%20Percent
  (if (<= (+ (Variables|Default|GetFirstPercent) (Variables|Default|GetSecondPercent) (Variables|Default|GetThirdPercent)) 99)
    (Variables|Default|SetIsOver? false)
    (else
      (Variables|Default|SetIsOver? true))))

(event EventBeginPlay)

(event Collision|EventActorBeginOverlap
  (params (OtherActor :type Actor%20Object%20Reference)))

(event EventTick
  (params (DeltaSeconds :type Float%20%28single-precision%29))
  (bind _progressmi3 (Variables|Default|GetProgressMI3))
  (bind _secondname (Variables|Default|GetSecondName))
  (bind _thirdname (Variables|Default|GetThirdName))
  (bind _progressmi1 (Variables|Default|GetProgressMI1))
  (bind _progressmi2 (Variables|Default|GetProgressMI2))
  (bind _drinkname (Variables|Default|GetDrinkName))
  (bind _drinkscolormap (Variables|Default|GetDrinksColorMap))
  (bind _value (Utilities|Map|Find _drinkscolormap _drinkname))
  (bind _returnvalue (Math|Conversions|ToLinearColor(Color) _value))
  (if (Variables|Default|GetIsClicked)
    (if (<= (Variables|Default|GetDrinkNum) 0)
      (Variables|Default|SetBar1Color _returnvalue)
      (bind _totalper (CallFunction|SetNameText (Variables|Default|GetFirstName) (+ (Variables|Default|GetBar1Percent) 0.0031) (Utilities|Text|ToText(Name) _drinkname)))
      (Variables|Default|SetFirstPercent _totalper)
      (Rendering|Material|SetVectorParameterValue _progressmi1 "ProgressColor1" (Variables|Default|GetBar1Color) :!class /Script/Engine.MaterialInstanceDynamic)
      (Rendering|Material|SetScalarParameterValue _progressmi1 "Progress" (+ (Variables|Default|GetBar1Percent) 0.0031) :!class /Script/Engine.MaterialInstanceDynamic)
      (CallFunction|SetNameLocation (Variables|Default|GetFirstName))
      (Variables|Default|SetBar1Percent (+ (Variables|Default|GetBar1Percent) 0.0031))
      (Rendering|Material|SetVectorParameterValue _progressmi2 "ProgressColor1" (Utilities|Struct|MakeLinearColor (.R (Utilities|Struct|BreakLinearColor (Variables|Default|GetBar2Color))) (.G (Utilities|Struct|BreakLinearColor (Variables|Default|GetBar2Color))) (.B (Utilities|Struct|BreakLinearColor (Variables|Default|GetBar2Color))) 3.0) :!class /Script/Engine.MaterialInstanceDynamic :!label _label) ; percent 설정 후 여기로
      (Rendering|Material|SetScalarParameterValue _progressmi2 "Progress" (+ (Variables|Default|GetBar2Percent) 0.0031) :!class /Script/Engine.MaterialInstanceDynamic)
      (CallFunction|SetNameLocation (Variables|Default|GetSecondName))
      (Variables|Default|SetBar2Percent (+ (Variables|Default|GetBar2Percent) 0.0031))
      (Rendering|Material|SetVectorParameterValue _progressmi3 "ProgressColor1" (Utilities|Struct|MakeLinearColor (.R (Utilities|Struct|BreakLinearColor (Variables|Default|GetBar3Color))) (.G (Utilities|Struct|BreakLinearColor (Variables|Default|GetBar3Color))) (.B (Utilities|Struct|BreakLinearColor (Variables|Default|GetBar3Color))) 6.0) :!class /Script/Engine.MaterialInstanceDynamic :!label _label_2)
      (Rendering|Material|SetScalarParameterValue _progressmi3 "Progress" (+ (Variables|Default|GetBar3Percent) 0.0031) :!class /Script/Engine.MaterialInstanceDynamic)
      (CallFunction|SetNameLocation (Variables|Default|GetThirdName))
      (Variables|Default|SetBar3Percent (+ (Variables|Default|GetBar3Percent) 0.0031))
      (elif (<= (Variables|Default|GetDrinkNum) 1)
        (Variables|Default|SetBar2Color _returnvalue)
        (Rendering|SetVisibility _secondname true false)
        (bind _totalper_2 (CallFunction|SetNameText _secondname (- (+ (Variables|Default|GetBar2Percent) 0.0031) (Variables|Default|GetBar1Percent)) (Utilities|Text|ToText(Name) _drinkname)))
        (Variables|Default|SetSecondPercent _totalper_2)
        (goto _label)
        (elif (<= (Variables|Default|GetDrinkNum) 2)
          (Variables|Default|SetBar3Color _returnvalue)
          (Rendering|SetVisibility _thirdname true false)
          (bind _totalper_3 (CallFunction|SetNameText _thirdname (- (+ (Variables|Default|GetBar3Percent) 0.0031) (Variables|Default|GetBar2Percent)) (Utilities|Text|ToText(Name) _drinkname)))
          (Variables|Default|SetThirdPercent _totalper_3)
          (goto _label_2))))))

(fn ConstructionScript
  (bind _returnvalue (Rendering|Material|CreateDynamicMaterialInstance (Variables|Default|GetProgressBar) 0 "/Game/Interface/MI_PBar1.MI_PBar1" :!class /Script/Engine.PrimitiveComponent))
  (Variables|Default|SetProgressMI1 _returnvalue)
  (bind _returnvalue_2 (Rendering|Material|CreateDynamicMaterialInstance (Variables|Default|GetProgressBar2) 0 "/Game/Interface/MI_PBar2.MI_PBar2" :!class /Script/Engine.PrimitiveComponent))
  (Variables|Default|SetProgressMI2 _returnvalue_2)
  (bind _returnvalue_3 (Rendering|Material|CreateDynamicMaterialInstance (Variables|Default|GetProgressBar3) 0 "/Game/Interface/MI_PBar3.MI_PBar3" :!class /Script/Engine.PrimitiveComponent))
  (Variables|Default|SetProgressMI3 _returnvalue_3))

(fn SetNameLocation
  (params (Alcohol%20Text :type Text%20Render%20Component%20Object%20Reference))
  (bind _returnvalue (Transformation|GetWorldLocation Alcohol%20Text))
  (bind (_x _y _z) (Math|Vector|BreakVector _returnvalue))
  (CallFunction|CheckPercent)
  (if (Variables|Default|GetIsOver?)
    (Variables|Default|SetIsClicked false)
    (else
      (Transformation|SetWorldLocation Alcohol%20Text (Math|Vector|MakeVector _x _y (+ _z 0.25)) false false))))

(fn SetNameText
  (params (Text :type Text%20Render%20Component%20Object%20Reference) (Alcohol%20Percent :type Float%20%28single-precision%29) (Alcohol%20Name :type Text))
  (bind _returnvalue (* Alcohol%20Percent 102.5))
  (bind _returnvalue_2 (Math|Float|Truncate _returnvalue))
  (CallFunction|CheckPercent)
  (if (Variables|Default|GetIsOver?)
    (Variables|Default|SetIsClicked false)
    (else
      (Rendering|Components|TextRender|SetText Text (Utilities|Text|FormatText "{Alcohol Name} {Percent}%" Alcohol%20Name _returnvalue_2))
      (return _returnvalue_2))))