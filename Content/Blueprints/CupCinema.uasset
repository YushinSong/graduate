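; Drink-pouring Blueprint where keys 1-3 pick a drink and holding left mouse pours it into a BP_Cup until release.
; DrawDrink tints and activates the drink's particle system plus FakeParticle, records pour order and colors, and the cup receives the drink data.
; Percentage-based color blending functions exist, but their EventGraph calls are disconnected and never run.
; Key 0 adds a Flex component at the static mesh's transform.
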(event EventBeginPlay
  (Components|Activation|Deactivate (Variables|Default|GetParticleSystem1)))

(event EventTick
  (params (DeltaSeconds :type Float%20%28single-precision%29)))

(event Input|KeyboardEvents|0
  (params (Key :type Key%20Structure))
  (:Pressed
    (AddComponent|AddFlexComponent true (Transformation|GetWorldTransform (Variables|Default|GetStaticMesh)))))

(event Input|MouseEvents|LeftMouseButton
  (params (Key :type Key%20Structure))
  (:Pressed
    (bind _asbp_cup (Utilities|Casting|CastToBP_Cup (Variables|Default|GetCup)))
    (if (Variables|/Game/Alcohol/BP_Cup.BP_Cup_C|GetIsOver? _asbp_cup)
      (Variables|/Game/Alcohol/BP_Cup.BP_Cup_C|SetIsClicked _asbp_cup false :!label _label)
      (Components|Activation|Deactivate (Variables|Default|GetParticleSystem2))
      (Variables|Default|SetIsPouring false)
      (else
        (Variables|/Game/Alcohol/BP_Cup.BP_Cup_C|SetIsClicked _asbp_cup true)
        (bind _returndrinkname (CallFunction|DrawDrink))
        (Variables|/Game/Alcohol/BP_Cup.BP_Cup_C|SetDrinkNum _asbp_cup (Variables|Default|GetWhatDrink?))
        (Variables|/Game/Alcohol/BP_Cup.BP_Cup_C|SetDrinkName _asbp_cup _returndrinkname)
        (Variables|/Game/Alcohol/BP_Cup.BP_Cup_C|SetDrinksColorMap _asbp_cup (Variables|Default|GetDrinksColorMap))
        (Variables|Default|SetIsPouring true))))
  (:Released
    (goto _label)))

(event Input|KeyboardEvents|1
  (params (Key :type Key%20Structure))
  (:Pressed
    (Variables|Default|SetWhatDrink? 0) ; default = 0
  ))

(event Input|KeyboardEvents|2
  (params (Key :type Key%20Structure))
  (:Pressed
    (Variables|Default|SetWhatDrink? 1)))

(event Input|KeyboardEvents|3
  (params (Key :type Key%20Structure))
  (:Pressed
    (Variables|Default|SetWhatDrink? 2)))

(fn ConstructionScript)

(fn DrawDrink
  (bind _activateddrinkcolors (Variables|Default|GetActivatedDrinkColors))
  (bind _drinks (Variables|Default|GetDrinks))
  (bind _drinkscolormap (Variables|Default|GetDrinksColorMap))
  (bind _whatdrink_ (Variables|Default|GetWhatDrink?))
  (bind _particlesystem2 (Variables|Default|GetParticleSystem2))
  (bind _particlesystem1 (Variables|Default|GetParticleSystem1))
  (bind _particlesystem3 (Variables|Default|GetParticleSystem3))
  (bind _output (Utilities|Array|Get(acopy) _drinks _whatdrink_))
  (bind (_value _returnvalue) (Utilities|Map|Find _drinkscolormap _output))
  (bind _returnvalue_2 (Math|Conversions|ToLinearColor(Color) _value))
  (Utilities|Array|AddUnique (Variables|Default|GetActivatedOrder) _whatdrink_)
  (if _returnvalue
    (switch int (Variables|Default|GetWhatDrink?)
      (:0
        (Effects|Components|ParticleSystem|SetColorParameter _particlesystem1 "InstanceColorScaleOverLife" _returnvalue_2)
        (Components|Activation|Activate _particlesystem1 false))
      (:1
        (Effects|Components|ParticleSystem|SetColorParameter _particlesystem2 "InstanceColorScaleOverLife" _returnvalue_2)
        (Components|Activation|Activate _particlesystem2 false))
      (:2
        (Effects|Components|ParticleSystem|SetColorParameter _particlesystem3 "InstanceColorScaleOverLife" _returnvalue_2)
        (Components|Activation|Activate _particlesystem3 false)))
    (if (== (Utilities|Array|FindItem _activateddrinkcolors _value) -1)
      (Utilities|Array|Add _activateddrinkcolors _value)
      (Variables|Default|SetPriviousColor (Variables|Default|GetLastColor)))
    (return _output)))

(fn WhatIsLastColor?
  (bind _activateddrinkcolors (Variables|Default|GetActivatedDrinkColors))
  (Variables|Default|SetLastColor (Math|Conversions|ToColor(LinearColor) (Math|Color|Lerp(LinearColor) (Math|Conversions|ToLinearColor(Color) (Variables|Default|GetPriviousColor)) (Math|Conversions|ToLinearColor(Color) (Utilities|Array|Get(acopy) _activateddrinkcolors (Utilities|Array|LastIndex _activateddrinkcolors))) (Utilities|Array|Get(acopy) (Variables|Default|GetDrinksPercent) (Variables|Default|GetWhichPercent?))))))

(fn PercentOfDrinks
  (params (Num :type Integer))
  (bind _drinkspercent (Variables|Default|GetDrinksPercent))
  (bind _drinkstime (Variables|Default|GetDrinksTime))
  (if (Variables|Default|GetIsPouring)
    (Variables|Default|SetTotalPouredTime (+ (Variables|Default|GetTotalPouredTime) 1.0))
    (Utilities|Array|SetArrayElem _drinkstime Num (+ (Utilities|Array|Get(acopy) _drinkstime Num) 1.0))
    (for (_ _array_index) _drinkspercent
      (Utilities|Array|SetArrayElem _drinkspercent _array_index (/ (Utilities|Array|Get(acopy) (Variables|Default|GetDrinksTime) _array_index) (Variables|Default|GetTotalPouredTime))))))

(fn NewColorChange
  (params (NewParam :type Particle%20System%20Component%20Object%20Reference))
  (Effects|Components|ParticleSystem|SetColorParameter NewParam "InstanceColorScaleOverLife" (Math|Conversions|ToLinearColor(Color) (Variables|Default|GetLastColor))))

(fn NumberOfDrinks
  (bind _activateddrinkcolors (Variables|Default|GetActivatedDrinkColors))
  (switch int (Utilities|Array|LastIndex _activateddrinkcolors)
    (:0
      (Variables|Default|SetPriviousColor (Utilities|Array|Get(acopy) _activateddrinkcolors)))
    (:1
      (bind _newparam (CallFunction|ReturnParticle))
      (CallFunction|NewColorChange _newparam)
      (bind _newparam_2 (CallFunction|ReturnParticle 1))
      (CallFunction|NewColorChange _newparam_2)
      (Variables|Default|SetWhichPercent? 1))
    (:2
      (bind _newparam_3 (CallFunction|ReturnParticle))
      (CallFunction|NewColorChange _newparam_3)
      (bind _newparam_4 (CallFunction|ReturnParticle 1))
      (CallFunction|NewColorChange _newparam_4)
      (bind _newparam_5 (CallFunction|ReturnParticle 2))
      (CallFunction|NewColorChange _newparam_5)
      (Variables|Default|SetWhichPercent? 2))))

(fn ReturnParticle
  (params (Num :type Integer))
  (switch int (Utilities|Array|Get(acopy) (Variables|Default|GetActivatedOrder) Num)
    (:0
      (return (Variables|Default|GetParticleSystem1)))
    (:1
      (return (Variables|Default|GetParticleSystem2)))
    (:2
      (return (Variables|Default|GetParticleSystem3)))))